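; BP_DataCore is a spinning pickup that the player collects by holding interact, which triggers the game's alarm.
; Tick rotates the actor and counter-rotates InnerCube, then shows the HUD interact prompt within range and accumulates hold progress, resetting it on release.
; On completion, it sets the player's HasDataCore flag, calls TriggerAlarm on the game mode, spawns a Niagara spark burst, and hides itself and the prompt.
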(event Custom|OnDataCoreCollected
  ;[0.15 0.15 0.15 0.5] On Collected — Set Alarm, Hide Core, Spawn VFX, Trigger Game Mode
  (Variables|Default|SetbAlarmTriggered true)
  (bind _asbp_third_person_character (Utilities|Casting|CastToBP_ThirdPersonCharacter (Game|GetPlayerCharacter 0)))
  (Variables|/Game/ThirdPerson/Blueprints/BP_ThirdPersonCharacter.BP_ThirdPersonCharacter_C|SetbHasDataCore _asbp_third_person_character true)
  (bind _asbp_game_mode_cz (Utilities|Casting|CastToBP_GameMode_CZ (Game|GetGameMode)))
  (Default|TriggerAlarm _asbp_game_mode_cz)
  (Niagara|SpawnSystematLocation "/Game/NiagaraExamples/FX_Sparks/NS_Spark_Burst.NS_Spark_Burst" (Transformation|GetActorLocation) "0, 0, 0" "0.500000,0.500000,0.500000")
  (Rendering|SetActorHiddenInGame true)
  (bind _asbp_game_mode_cz_2 (Utilities|Casting|CastToBP_GameMode_CZ (Game|GetGameMode)))
  (Widget|SetVisibility (Variables|/Game/ChronosZero/Blueprints/UI/WBP_HUD.WBP_HUD_C|GetInteractPrompt (Variables|/Game/ChronosZero/Blueprints/Systems/BP_GameMode_CZ.BP_GameMode_CZ_C|GetHUDWidget _asbp_game_mode_cz_2)) "Hidden"))

(event EventTick
  (params (DeltaSeconds :type Float%20%28single-precision%29))
  ;[0.15 0.15 0.15 0.5] Data Core Spin Animation — Outer and Inner Rotation
  (Class|Actor|AddActorWorldRotation (Math|Rotator|MakeRotator (* DeltaSeconds 45.0) (* DeltaSeconds 63.0) (* DeltaSeconds 9e+01)))
  (Transformation|AddRelativeRotation (Variables|Default|GetInnerCube) (Math|Rotator|MakeRotator (* DeltaSeconds -45.0) (* DeltaSeconds -63.0) (* DeltaSeconds -9e+01)) false false)
  (if (not (Variables|Default|GetbAlarmTriggered))
    ;[0.15 0.15 0.15 0.5] Interact System — Proximity Check, Hold Progress, Trigger on Complete and Interact Prompt — Show When Close, Hide When Far
    (if (< (Transformation|GetDistanceTo (Game|GetPlayerCharacter 0)) 3e+02)
      (bind _asbp_game_mode_cz (Utilities|Casting|CastToBP_GameMode_CZ (Game|GetGameMode)))
      (Widget|SetVisibility (Variables|/Game/ChronosZero/Blueprints/UI/WBP_HUD.WBP_HUD_C|GetInteractPrompt (Variables|/Game/ChronosZero/Blueprints/Systems/BP_GameMode_CZ.BP_GameMode_CZ_C|GetHUDWidget _asbp_game_mode_cz)) "Visible")
      (bind _asbp_third_person_character (Utilities|Casting|CastToBP_ThirdPersonCharacter (Game|GetPlayerCharacter 0)))
      (if (Variables|/Game/ThirdPerson/Blueprints/BP_ThirdPersonCharacter.BP_ThirdPersonCharacter_C|GetbIsInteracting _asbp_third_person_character)
        (Variables|Default|SetInteractProgress (+ (Variables|Default|GetInteractProgress) DeltaSeconds))
        (if (>= (Variables|Default|GetInteractProgress) (Variables|Default|GetInteractDuration))
          (CallFunction|OnDataCoreCollected))
        (else
          (Variables|Default|SetInteractProgress 0.0)))
      (else
        (bind _asbp_game_mode_cz_2 (Utilities|Casting|CastToBP_GameMode_CZ (Game|GetGameMode)))
        (Widget|SetVisibility (Variables|/Game/ChronosZero/Blueprints/UI/WBP_HUD.WBP_HUD_C|GetInteractPrompt (Variables|/Game/ChronosZero/Blueprints/Systems/BP_GameMode_CZ.BP_GameMode_CZ_C|GetHUDWidget _asbp_game_mode_cz_2)) "Hidden")))))

(fn ConstructionScript)