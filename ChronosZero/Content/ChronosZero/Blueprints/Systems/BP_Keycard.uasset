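; BP_Keycard is a keycard pickup that grants the player character keycard possession and spins in the world until collected.
; A timeline started on BeginPlay drives the actor's yaw.
; On overlap with BP_ThirdPersonCharacter, a Collected flag guards a single pickup that sets the character's HasKeycard flag, then hides, disables collision on and destroys the actor.
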(event EventBeginPlay
  (bind _yaw (Timeline|RotationTimeline Play)
    (:Update
      (Transformation|SetActorRotation (Math|Rotator|MakeRotator 0.0 0.0 _yaw)))))

(event Collision|EventActorBeginOverlap
  (params (OtherActor :type Actor%20Object%20Reference))
  (bind _asbp_third_person_character (Utilities|Casting|CastToBP_ThirdPersonCharacter OtherActor))
  (if (not (Variables|Default|GetbCollected))
    (Variables|Default|SetbCollected true)
    (Variables|/Game/ThirdPerson/Blueprints/BP_ThirdPersonCharacter.BP_ThirdPersonCharacter_C|SetbHasKeycard _asbp_third_person_character true)
    (Rendering|SetActorHiddenInGame true)
    (Collision|SetActorEnableCollision false)
    (Actor|DestroyActor)))

(fn ConstructionScript)