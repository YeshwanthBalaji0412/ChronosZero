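; Game mode for Chronos Zero that runs the HUD, alarm escape sequence and victory or game-over screens.
; TriggerAlarm plays a siren, camera shake and timeline light flicker, then turns point lights red, starts the timer, activates tagged sparks and slams the shutter.
; CountdownTick updates the HUD and shows game over at zero.
; End screens pause the game and show the cursor; R opens the main menu.
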(event Custom|TriggerAlarm
  ;[0.15 0.15 0.15 0.5] Alarm Trigger — Set Active, Play Siren, Camera Shake, Start Flicker and Light Flicker — Change All Point Lights to Red on Alarm
  (Variables|Default|SetbAlarmActive true)
  (Audio|PlaySound2D "/Game/CyberwavePack/Sounds/Sounds/S_Scarlet_Virus_Dplr.S_Scarlet_Virus_Dplr" 1.0 1.0 0.0 0 0)
  (Game|Feedback|ClientStartCameraShake (Game|GetPlayerController 0) "/Game/ChronosZero/Blueprints/Systems/BP_AlarmCameraShake.BP_AlarmCameraShake_C" 1.0 "CameraLocal" "0, 0, 0")
  (bind _intensity (Timeline|AlarmFlicker Play)
    (:Update
      (bind _outactors (Actor|GetAllActorsOfClass "/Script/Engine.PointLight"))
      (for _array_element _outactors
        (Rendering|Components|Light|SetIntensity (Variables|/Script/Engine.Light|GetLightComponent _array_element) _intensity)))
    (:Finished
      (bind _outactors_2 (Actor|GetAllActorsOfClass "/Script/Engine.PointLight"))
      (for _array_element_2 _outactors_2
        (bind _aspoint_light (Utilities|Casting|CastToPointLight _array_element_2))
        (Rendering|Components|Light|SetLightColor (Variables|/Script/Engine.Light|GetLightComponent _aspoint_light) "(R=1.000000,G=0.000000,B=0.000000,A=1.000000)" true)
        (Rendering|Components|Light|SetIntensity (Variables|/Script/Engine.Light|GetLightComponent _aspoint_light) 5e+03))
      ;[0.15 0.15 0.15 0.5] Countdown Start — Start Timer, Show HUD Timer, Activate Spark VFX and Door Slam — Hide Placeholder, Animate Door Closing on Alarm
      (Utilities|Time|SetTimerbyEvent (EventDispatchers|CreateEvent :!event CountdownTick) 1.0 true)
      (Default|ShowTimer (Variables|Default|GetHUDWidget))
      (bind _outactors_3 (Actor|GetAllActorswithTag "AlarmSpark"))
      (for _array_element_3 _outactors_3
        (bind _asniagara_particle_system_actor (Utilities|Casting|CastToNiagaraActor _array_element_3))
        (Components|Activation|Activate (Variables|/Script/Niagara.NiagaraActor|GetNiagaraComponent _asniagara_particle_system_actor) true))
      (bind _outactors_4 (Actor|GetAllActorswithTag "ShutterDoor"))
      (Rendering|SetActorHiddenInGame (Utilities|Array|Get(acopy) _outactors_4) false)
      (bind _slam (Timeline|DoorSlam PlayFromStart)
        (:Update
          (Transformation|SetActorLocation (Utilities|Array|Get(acopy) _outactors_4) (Math|Vector|MakeVector 6.25e+03 -7.2e+02 _slam) false false))))))

(event EventBeginPlay
  ;[0.15 0.15 0.15 0.5] HUD Setup — Create and Display WBP_HUD on Game Start
  (bind _returnvalue (UserInterface|CreateWidget "/Game/ChronosZero/Blueprints/UI/WBP_HUD.WBP_HUD_C" (Game|GetPlayerController 0)))
  (bind _output_get (Variables|Default|SetHUDWidget _returnvalue))
  (UserInterface|Viewport|AddtoViewport _output_get 0))

(event Input|KeyboardEvents|R
  (params (Key :type Key%20Structure))
  (:Pressed
    (Game|OpenLevel(byName) "L_MainMenu")))

(fn ConstructionScript)

(fn CountdownTick
  (bind _output_get (Variables|Default|SetCountdownTime (- (Variables|Default|GetCountdownTime) 1.0)))
  (Default|UpdateTimer (Variables|Default|GetHUDWidget) _output_get)
  (if (<= (Variables|Default|GetCountdownTime) 0.0)
    (bind _asbp_game_mode_cz (Utilities|Casting|CastToBP_GameMode_CZ (Game|GetGameMode)))
    (CallFunction|ShowGameOver _asbp_game_mode_cz)))

(fn ShowVictory
  (bind _returnvalue (UserInterface|CreateWidget "/Game/ChronosZero/Blueprints/UI/WBP_Victory.WBP_Victory_C" (Game|GetPlayerController 0)))
  (UserInterface|Viewport|AddtoViewport _returnvalue 0)
  (Game|SetGamePaused true)
  (Variables|/Script/Engine.PlayerController|SetbShowMouseCursor (Game|GetPlayerController 0) true))

(fn ShowGameOver
  (bind _returnvalue (UserInterface|CreateWidget "/Game/ChronosZero/Blueprints/UI/WBP_GameOver.WBP_GameOver_C" (Game|GetPlayerController 0)))
  (UserInterface|Viewport|AddtoViewport _returnvalue 0)
  (Game|SetGamePaused true)
  (Variables|/Script/Engine.PlayerController|SetbShowMouseCursor (Game|GetPlayerController 0) true))