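; BP_Door_Z2Z3 is a keycard door, apparently between zones 2 and 3, that slides upward once and stays open.
; Tick polls player distance and opens the door when a nearby BP_ThirdPersonCharacter has the keycard.
; The DoorSlide timeline lerps the mesh up from its BeginPlay position, guarded by IsOpen.
; OpenDoor triggers the same slide without a keycard check; overlap events set PlayerInRange, which this graph never reads.
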(event Custom|OpenDoor
  (if (not (Variables|Default|GetbIsOpen))
    (Variables|Default|SetbIsOpen true)
    (bind _alpha (Timeline|DoorSlide PlayFromStart)
      (:Update
        (Transformation|SetRelativeLocation (Variables|Debug|GetStaticMeshComponent) (Math|Vector|Lerp(Vector) (Variables|Default|GetClosedLocation) (+ (Variables|Default|GetClosedLocation) (Math|Vector|MakeVector 0.0 0.0 6e+02)) _alpha) false false)))))

(event EventBeginPlay
  (Variables|Default|SetClosedLocation (Variables|/Script/Engine.SceneComponent|GetRelativeLocation (Variables|Debug|GetStaticMeshComponent))))

(event Collision|EventActorBeginOverlap
  (params (OtherActor :type Actor%20Object%20Reference))
  (Utilities|Casting|CastToBP_ThirdPersonCharacter OtherActor)
  (Variables|Default|SetbPlayerInRange true))

(event EventTick
  (params (DeltaSeconds :type Float%20%28single-precision%29))
  (if (< (Transformation|GetDistanceTo (Game|GetPlayerCharacter 0)) 4e+02)
    (bind _asbp_third_person_character (Utilities|Casting|CastToBP_ThirdPersonCharacter (Game|GetPlayerCharacter 0)))
    (if (Variables|/Game/ThirdPerson/Blueprints/BP_ThirdPersonCharacter.BP_ThirdPersonCharacter_C|GetbHasKeycard _asbp_third_person_character)
      (if (not (Variables|Default|GetbIsOpen))
        (Variables|Default|SetbIsOpen true)
        (bind _alpha (Timeline|DoorSlide PlayFromStart)
          (:Update
            (Transformation|SetRelativeLocation (Variables|Debug|GetStaticMeshComponent) (Math|Vector|Lerp(Vector) (Variables|Default|GetClosedLocation) (+ (Variables|Default|GetClosedLocation) (Math|Vector|MakeVector 0.0 0.0 6e+02)) _alpha) false false)))))))

(event Collision|EventActorEndOverlap
  (params (OtherActor :type Actor%20Object%20Reference))
  (Utilities|Casting|CastToBP_ThirdPersonCharacter OtherActor)
  (Variables|Default|SetbPlayerInRange false))

(fn ConstructionScript)