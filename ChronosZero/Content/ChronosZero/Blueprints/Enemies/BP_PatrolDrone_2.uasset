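; Patrol drone enemy that loops through patrol points and triggers game over when it keeps the player detected long enough.
; Each Tick checks a forward dot-product cone, range and a random roll against the player's DetectionModifier; the line trace result is unused.
; Detection swaps the cone to an alert material, starts a chase and runs a timer, which a failed roll resets.
; An active GameMode alarm raises speed and sends it after the player.
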(event Custom|MoveToNextPoint
  ;[0.15 0.15 0.15 0.5] Patrol AI — Move Between Points, Cycle on Arrival
  (AI|AIMoveTo self (Transformation|GetActorLocation (Utilities|Array|Get(acopy) (Variables|Default|GetPatrolPoints) (Variables|Default|GetCurrentPatrolIndex))) 0 5.0 false
    (:OnSuccess
      (Variables|Default|SetCurrentPatrolIndex (Math|Integer|%(Integer) (+ (Variables|Default|GetCurrentPatrolIndex) 1) (Utilities|Array|Length (Variables|Default|GetPatrolPoints))))
      (CallFunction|MovetoNextPoint))))

(event Custom|OnPlayerDetected
  ;[0.15 0.15 0.15 0.5] Vision Detection — dot product + line trace + DetectionModifier
  (if (not (Variables|Default|GetbPlayerInCone))
    (Variables|Default|SetbPlayerInCone true)
    (Rendering|Material|SetMaterial (Variables|Default|GetVisionConeMesh) 0 "/Game/ChronosZero/Blueprints/Enemies/Materials/M_VisionCone_Alert.M_VisionCone_Alert")
    (AI|AIMoveTo self "0, 0, 0" (Game|GetPlayerCharacter 0) 5.0 false)))

(event EventBeginPlay
  ;[0.15 0.15 0.15 0.5] Patrol AI — Move Between Points, Cycle on Arrival
  (CallFunction|MovetoNextPoint))

(event EventTick
  (params (DeltaSeconds :type Float%20%28single-precision%29))
  (bind _returnvalue (Game|GetPlayerCharacter 0))
  (bind _returnvalue_2 (Transformation|GetActorLocation _returnvalue))
  ;[0.15 0.15 0.15 0.5] Vision Detection — dot product + line trace + DetectionModifier
  (bind _asbp_game_mode_cz (Utilities|Casting|CastToBP_GameMode_CZ (Game|GetGameMode)))
  (if (Variables|/Game/ChronosZero/Blueprints/Systems/BP_GameMode_CZ.BP_GameMode_CZ_C|GetbAlarmActive _asbp_game_mode_cz)
    (Variables|/Script/Engine.FloatingPawnMovement|SetMaxSpeed (Variables|Default|GetFloatingPawnMovement) 5e+02)
    (Variables|Default|SetbCanDetect true)
    (AI|AIMoveTo self "0, 0, 0" (Game|GetPlayerCharacter 0) 5.0 false
      (:OnSuccess
        _)
      (:OnFail
        _))
    (CallFunction|MovetoNextPoint)
    (else
      (Variables|/Script/Engine.FloatingPawnMovement|SetMaxSpeed (Variables|Default|GetFloatingPawnMovement) 2e+02)))
  (if (Variables|Default|GetbCanDetect)
    (if (> (Math|Vector|DotProduct (Transformation|GetActorForwardVector) (Math|Vector|GetUnitDirection(Vector) (Transformation|GetActorLocation self) _returnvalue_2)) 0.7)
      (if (< (Transformation|GetDistanceTo _returnvalue) (Variables|Default|GetVisionRange))
        (bind _outhit (Collision|LineTraceByChannel (+ (Transformation|GetActorLocation) (Math|Vector|MakeVector 0.0 0.0 5e+01)) (+ _returnvalue_2 (Math|Vector|MakeVector 0.0 0.0 6e+01)) "TraceTypeQuery1" false 0 "None" true "(R=1.000000,G=0.000000,B=0.000000,A=1.000000)" "(R=0.000000,G=1.000000,B=0.000000,A=1.000000)" 0.0))
        (bind _asbp_third_person_character (Utilities|Casting|CastToBP_ThirdPersonCharacter _returnvalue))
        (if (< (Math|Random|RandomFloatinRange 0.0 1.0) (Variables|/Game/ThirdPerson/Blueprints/BP_ThirdPersonCharacter.BP_ThirdPersonCharacter_C|GetDetectionModifier _asbp_third_person_character))
          (CallFunction|OnPlayerDetected)
          (if (Variables|Default|GetbPlayerInCone)
            (bind _output_get (Variables|Default|SetDetectionTimer (+ (Variables|Default|GetDetectionTimer) DeltaSeconds)))
            (if (>= _output_get 2.0)
              (bind _asbp_game_mode_cz_2 (Utilities|Casting|CastToBP_GameMode_CZ (Game|GetGameMode)))
              (Default|ShowGameOver _asbp_game_mode_cz_2)))
          (elif (Variables|Default|GetbPlayerInCone)
            (Variables|Default|SetbPlayerInCone false)
            (Variables|Default|SetDetectionTimer 0.0)
            (Components|Movement|StopMovementImmediately (Variables|Default|GetFloatingPawnMovement))
            (Rendering|Material|SetMaterial (Variables|Default|GetVisionConeMesh) 0 "/Game/ChronosZero/Blueprints/Enemies/Materials/M_VisionCone.M_VisionCone")
            (CallFunction|MovetoNextPoint)))))))

(fn ConstructionScript)